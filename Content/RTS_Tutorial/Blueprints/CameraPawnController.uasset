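; RTS player controller that drives the camera pawn and handles building placement.
; On BeginPlay it spawns a construction manager and ghost building, then creates the main HUD.
; Input moves the camera by axes or screen edges, pans and zooms it, with axis speed scaled by zoom and Shift boosting movement.
; In build mode the ghost follows the cursor each tick, and left-click queues non-overlapping placements with the manager.
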(event `self.ReceiveTick`
  (params (DeltaSeconds :type "Float (single-precision)"))
  ;[1 1 1] Tick
  (if (`self.BuildModeActive`)
    (if (!= (`self.GhostBuildingRef`) null)
      (`/Game/RTS_Tutorial/Blueprints/Buildings/GhostBuilding_BP.SetCursorPosition` (`self.GhostBuildingRef`) (`/Game/RTS_Tutorial/Libraries/FunctionLibrary.SetCursorWorldPosition` self (`self.SetSightDistance`))))))

(event `InputAction|Deselect`
  (params (Key :type "Key Structure"))
  ;[1 1 1] Comment
  (:`Pressed`
    (if (`self.BuildModeActive`)
      (`/Game/RTS_Tutorial/Blueprints/Buildings/GhostBuilding_BP.KillGhost` (`self.GhostBuildingRef`))
      (set `self.BuildModeActive` false))))

(event `self.ReceiveBeginPlay`
  (bind _returnvalue (`KismetMathLibrary.MakeTransform` (0.0 0.0 0.0)))
  ;[1 1 1] Begin Play
  (`|ExecutionSequence`
    (:`then_0`
      (`self.ReferenceCasts`))
    (:`then_1`
      (bind _returnvalue_2 (`|SpawnActorFromClass` "/Game/RTS_Tutorial/Blueprints/Constructions/ConstructionManger_BP.ConstructionManger_BP_C" _returnvalue "AlwaysSpawn" "OverrideRootScale" null null))
      (set `self.ConstructionManagerRef` _returnvalue_2))
    (:`then_2`
      (bind _returnvalue_3 (`|SpawnActorFromClass` "/Game/RTS_Tutorial/Blueprints/Buildings/GhostBuilding_BP.GhostBuilding_BP_C" _returnvalue "AlwaysSpawn" "OverrideRootScale" null self null))
      (set `self.GhostBuildingRef` _returnvalue_3))
    (:`then_3`
      (`WidgetBlueprintLibrary.SetInputMode_GameAndUIEx` self null "LockInFullscreen" false)
      (`self.CreateHIUDs`)
      (`UserWidget.AddToViewport` (`self.MainHUDRef`) 0))))

(event `Key|LeftMouseButton`
  (params (Key :type "Key Structure"))
  ;[1 1 1] LeftMouseButton
  (:`Pressed`
    (if (and (`self.BuildModeActive`) (not (`/Game/RTS_Tutorial/Blueprints/Buildings/GhostBuilding_BP.CheckOverlap` (`self.GhostBuildingRef`))))
      (bind _constructionstruct (`/Game/RTS_Tutorial/Blueprints/Buildings/GhostBuilding_BP.GetConstructionStruct` (`self.GhostBuildingRef`)))
      (`/Game/RTS_Tutorial/Blueprints/Constructions/ConstructionManger_BP.QueueConstruction` (`self.ConstructionManagerRef`) _constructionstruct)
      (`/Game/RTS_Tutorial/Blueprints/Buildings/GhostBuilding_BP.KillGhost` (`self.GhostBuildingRef`)))))

(event `InputAxis|MoveForward`
  (params (AxisValue :type "Float (single-precision)"))
  ;[1 1 1] CameraMovement
  ;;[1 1 1] Movement X
  (if (not (`self.DisableCamNav`))
    (`self.K2_SetActorTransform` (`self.CameraPawnRef`) (`self.MovementX` (`self.MovementSpeedCalculation`) (`self.FastMoveMultiplier`) AxisValue (`self.CameraPawnRef`)) false false)))

(event `InputAxis|MoveRight`
  (params (AxisValue :type "Float (single-precision)"))
  ;[1 1 1] CameraMovement
  ;;[1 1 1] Movement Y
  (if (not (`self.DisableCamNav`))
    (`self.K2_SetActorTransform` (`self.CameraPawnRef`) (`KismetMathLibrary.MakeTransform` (`KismetMathLibrary.MakeVector` (.x (.location (`self.MovementY` AxisValue (`self.MovementSpeedCalculation`) (`self.FastMoveMultiplier`) (`self.CameraPawnRef`)))) (.y (.location (`self.MovementY` AxisValue (`self.MovementSpeedCalculation`) (`self.FastMoveMultiplier`) (`self.CameraPawnRef`)))) 100.0) (.rotation (`self.MovementY` AxisValue (`self.MovementSpeedCalculation`) (`self.FastMoveMultiplier`) (`self.CameraPawnRef`))) (.scale (`self.MovementY` AxisValue (`self.MovementSpeedCalculation`) (`self.FastMoveMultiplier`) (`self.CameraPawnRef`)))) false false)))

(event `InputAxisKey|MouseX`
  (params (AxisValue :type "Float (single-precision)"))
  ;[1 1 1] CameraMovement
  ;;[1 1 1] Pan X
  (`/Engine/EditorBlueprintResources/StandardMacros.Gate` true :!label _label
    (:`Exit`
      (`self.K2_SetActorRotation` (`self.CameraPawnRef`) (`KismetMathLibrary.MakeRotator` (.roll (`self.K2_GetActorRotation` (`self.CameraPawnRef`))) (.pitch (`self.K2_GetActorRotation` (`self.CameraPawnRef`))) (+ (.yaw (`self.K2_GetActorRotation` (`self.CameraPawnRef`))) (* (`self.PanSensetivity`) AxisValue))) false))))

(event `InputAction|PanReset`
  (params (Key :type "Key Structure"))
  (bind _camerapawnref (`self.CameraPawnRef`))
  ;[1 1 1] CameraMovement
  ;;[1 1 1] Pan Reset
  (:`Pressed`
    (`self.K2_SetActorRotation` _camerapawnref (`KismetMathLibrary.MakeRotator` (.roll (`self.K2_GetActorRotation` _camerapawnref)) 0.0 (.yaw (`self.K2_GetActorRotation` _camerapawnref))) false)))

(event `InputAction|Pan`
  (params (Key :type "Key Structure"))
  ;[1 1 1] CameraMovement
  ;;[1 1 1] Pan X
  (:`Pressed`
    (set `self.DisableCamNav` true)
    (goto _label :!via `Open`))
  (:`Released`
    (set `self.DisableCamNav` false)
    (goto _label :!via `Close`)))

(event `Key|LeftShift`
  (params (Key :type "Key Structure"))
  ;[1 1 1] CameraMovement
  ;;[1 1 1] Move Multiplier
  (:`Pressed`
    (set `self.FastMoveMultiplier` 2.0))
  (:`Released`
    (set `self.FastMoveMultiplier` 1.0)))

(event `InputAxisKey|MouseY`
  (params (AxisValue :type "Float (single-precision)"))
  ;[1 1 1] CameraMovement
  ;;[1 1 1] Pan Y
  (`/Engine/EditorBlueprintResources/StandardMacros.Gate` true :!label _label_2
    (:`Exit`
      (`self.K2_SetActorRotation` (`self.CameraPawnRef`) (`KismetMathLibrary.MakeRotator` (.roll (`self.K2_GetActorRotation` (`self.CameraPawnRef`))) (`KismetMathLibrary.FClamp` (+ (.pitch (`self.K2_GetActorRotation` (`self.CameraPawnRef`))) (* (`self.PanSensetivity`) AxisValue)) -15.0 45.0) (.yaw (`self.K2_GetActorRotation` (`self.CameraPawnRef`)))) false))))

(event `InputAction|Pan`
  (params (Key :type "Key Structure"))
  ;[1 1 1] CameraMovement
  ;;[1 1 1] Pan Y
  (:`Pressed`
    (set `self.DisableCamNav` true)
    (goto _label_2 :!via `Open`))
  (:`Released`
    (set `self.DisableCamNav` false)
    (goto _label_2 :!via `Close`)))

(event `InputAction|ZoomReset`
  (params (Key :type "Key Structure"))
  ;[1 1 1] CameraMovement
  ;;[1 1 1] Zoom reset
  (:`Pressed`
    (set `SpringArmComponent.TargetArmLength` 1500.0 (`/Game/RTS_Tutorial/Blueprints/CameraPawn.SpringArm` (`self.CameraPawnRef`)))))

(event `InputAxisKey|MouseX`
  (params (AxisValue :type "Float (single-precision)"))
  ;[1 1 1] CameraMovement
  ;;[1 1 1] Edge Movement
  (if (not (`self.DisableCamNav`))
    (bind (_deltaxspeed _deltayspeed) (`self.ScreenEdgeMovement` :!label _label_3))
    (`self.K2_AddActorLocalOffset` (`self.CameraPawnRef`) (`KismetMathLibrary.MakeVector` _deltaxspeed _deltayspeed) true false)))

(event `InputAction|ZoomIn`
  (params (Key :type "Key Structure"))
  (bind _springarm (`/Game/RTS_Tutorial/Blueprints/CameraPawn.SpringArm` (`self.CameraPawnRef`)))
  ;[1 1 1] CameraMovement
  ;;[1 1 1] Zoom In/Out
  (:`Pressed`
    (set `SpringArmComponent.TargetArmLength` (`KismetMathLibrary.FClamp` (- (`SpringArmComponent.TargetArmLength` _springarm) (`self.ZoomSensitivity`)) 500.0 (`self.MaxArmDistance`)) _springarm)))

(event `InputAxisKey|MouseY`
  (params (AxisValue :type "Float (single-precision)"))
  ;[1 1 1] CameraMovement
  ;;[1 1 1] Edge Movement
  (if (not (`self.DisableCamNav`))
    (goto _label_3 :!via `MouseY`)))

(event `InputAction|ZoomOut`
  (params (Key :type "Key Structure"))
  (bind _springarm (`/Game/RTS_Tutorial/Blueprints/CameraPawn.SpringArm` (`self.CameraPawnRef`)))
  ;[1 1 1] CameraMovement
  ;;[1 1 1] Zoom In/Out
  (:`Pressed`
    (set `SpringArmComponent.TargetArmLength` (`KismetMathLibrary.FClamp` (+ (`SpringArmComponent.TargetArmLength` _springarm) (`self.ZoomSensitivity`) 0.0) 500.0 (`self.MaxArmDistance`)) _springarm)))

(fn `MovementSpeedCalculation`
  (returns (MoveSensetivity :type "Float (double-precision)"))
  (return (`KismetMathLibrary.FClamp` (/ (`SpringArmComponent.TargetArmLength` (`/Game/RTS_Tutorial/Blueprints/CameraPawn.SpringArm` (`self.CameraPawnRef`))) 100.0) 5.0 20.0)))

(fn `SetSightDistance`
  (returns (SightDistance :type "Float (double-precision)"))
  (return (+ (`self.SightDistance`) (`SpringArmComponent.TargetArmLength` (`/Game/RTS_Tutorial/Blueprints/CameraPawn.SpringArm` (`self.CameraPawnRef`))))))

(fn `UserConstructionScript`)