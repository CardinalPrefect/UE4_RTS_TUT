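; Ghost preview actor for RTS build mode, showing where a building would be placed.
; ConstructBuilding briefly spawns the building class to read its display mesh and construction proxy, then activates the ghost and flags build mode on the controller.
; While active, a gated Tick snaps the externally set cursor position to a grid and swaps to an error material on overlap.
; GetConstructionStruct packages class, proxy, mesh and transform for construction.
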(event `OnSpawn`
  (params (DisplayMesh :type "StaticMesh Object Reference") (BuildingClass :type "/Game/RTS_Tutorial/Blueprints/Buildings/BuildingMaster_BP Class Reference") (ConstructionProxy :type "/Game/RTS_Tutorial/Blueprints/Constructions/ConstructionProxy_BP Class Reference"))
  ;[1 1 1] On Spawn Ghost
  (if (not (`self.IsActive`))
    (set `self.BuildingClass` BuildingClass)
    (set `self.ConstructionProxy` ConstructionProxy)
    (set `self.DisplayMesh` DisplayMesh)
    (set `self.IsActive` true)
    (set `/Game/RTS_Tutorial/Blueprints/CameraPawnController.BuildModeActive` true (`self.ControllerRef`))
    (`StaticMeshComponent.SetStaticMesh` (`self.GhostBuilding_Mesh`) (`self.DisplayMesh`))
    (`self.OpenTickGate`)
    (`self.SetMaterial` (not (`self.IsOverlapping`)))))

(event `KillGhost`
  ;[1 1 1] Kill Ghost
  (set `self.BuildingClass` null)
  (set `self.ConstructionProxy` null)
  (`self.CloseTickGate`)
  (set `self.DisplayMesh` null)
  (set `self.IsActive` false)
  (set `/Game/RTS_Tutorial/Blueprints/CameraPawnController.BuildModeActive` false (`self.ControllerRef`))
  (`StaticMeshComponent.SetStaticMesh` (`self.GhostBuilding_Mesh`) (`self.DisplayMesh`)))

(event `/Game/RTS_Tutorial/Interfaces/I_HUD.ConstructBuilding`
  (params (MainBuilding :type "/Game/RTS_Tutorial/Blueprints/Buildings/BuildingMaster_BP Class Reference"))
  ;[1 1 1] Comment
  (bind _returnvalue (`|SpawnActorFromClass` MainBuilding (`KismetMathLibrary.MakeTransform` (0.0 0.0 0.0)) "Undefined" "OverrideRootScale" null (`self.ControllerRef`) null))
  (`|ExecutionSequence`
    (:`then_0`
      (bind _asbuilding_master_bp (castclass `/Game/RTS_Tutorial/Blueprints/Buildings/BuildingMaster_BP` MainBuilding))
      (`self.KillGhost`)
      (`self.OnSpawn` (`/Game/RTS_Tutorial/Blueprints/Buildings/BuildingMaster_BP.DisplayMesh` _returnvalue) _asbuilding_master_bp (`/Game/RTS_Tutorial/Blueprints/Buildings/BuildingMaster_BP.ConstructionProxy` _returnvalue)))
    (:`then_1`
      (`self.K2_DestroyActor` _returnvalue))))

(event `self.ReceiveTick`
  (params (DeltaSeconds :type "Float (single-precision)"))
  ;[1 1 1] Tick
  (`/Engine/EditorBlueprintResources/StandardMacros.Gate` true :!label _label
    (:`Exit`
      (`self.K2_SetActorLocation` self (`self.SetGridSpawnVector`) false false)
      (if (`self.CheckOverlap`)
        (`self.SetMaterial` true)
        (else
          (`self.SetMaterial` false))))))

(event `OpenTickGate`
  ;[1 1 1] Tick
  (goto _label :!via `Open`))

(event `CloseTickGate`
  ;[1 1 1] Tick
  (goto _label :!via `Close`))

(event `SetMaterial`
  (params (IsError :type Boolean))
  (bind _ghostbuilding_mesh (`self.GhostBuilding_Mesh`))
  ;[1 1 1] SetMaterial
  (if (not (== IsError (`self.IsOverlapping`)))
    (bind _output_get (set `self.IsOverlapping` IsError))
    (if _output_get
      (`PrimitiveComponent.SetMaterial` _ghostbuilding_mesh 0 "/Game/RTS_Tutorial/Materials/GhostError_M_Inst.GhostError_M_Inst")
      (else
        (`PrimitiveComponent.SetMaterial` _ghostbuilding_mesh 0 "/Game/RTS_Tutorial/Materials/Ghost_M_Inst.Ghost_M_Inst")))))

(fn `CheckOverlap`
  (returns (Overlapping :type Boolean))
  (return (> (`KismetArrayLibrary.Array_Length` (`self.GetOverlappingActors` "/Script/Engine.Actor")) 0)))

(fn `GetConstructionStruct`
  (returns (ConstructionStruct :type "/Game/RTS_Tutorial/Strucs/Construction_Struct Structure"))
  (return (make `/Game/RTS_Tutorial/Strucs/Construction_Struct` (`self.BuildingClass`) (`self.ConstructionProxy`) (`KismetMathLibrary.MakeTransform` (`self.K2_GetActorLocation`) (`self.K2_GetActorRotation`)) (`self.DisplayMesh`) 1.0)))

(fn `SetCalendar`
  (params (Date :type "Array of Integer (by ref)"))
  (returns (Success :type Boolean))
  (return false))

(fn `SetClock`
  (params (Time :type "Array of Integer (by ref)"))
  (returns (Success :type Boolean))
  (return false))

(fn `SetCursorPosition`
  (params (CursorLocation :type "Vector Structure"))
  (set `self.CursorWorldPosition` CursorLocation)
  (return))

(fn `SetGridSpawnVector`
  (returns (GridSnap :type "Vector Structure"))
  (bind (_cursorworldposition_x _cursorworldposition_y _cursorworldposition_z) (`KismetMathLibrary.BreakVector` (`self.CursorWorldPosition`)))
  (bind _gridsize (`self.GridSize`))
  (return (`KismetMathLibrary.MakeVector` (`/Game/RTS_Tutorial/Libraries/FunctionLibrary.GridSnap` _cursorworldposition_x _gridsize) (`/Game/RTS_Tutorial/Libraries/FunctionLibrary.GridSnap` _cursorworldposition_y _gridsize) (`/Game/RTS_Tutorial/Libraries/FunctionLibrary.GridSnap` _cursorworldposition_z _gridsize))))

(fn `UserConstructionScript`)